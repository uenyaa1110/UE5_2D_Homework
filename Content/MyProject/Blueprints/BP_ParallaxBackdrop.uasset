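; BP_ParallaxBackdrop is a side-scrolling backdrop actor that fakes depth with three parallax layers.
; BeginPlay records the player's starting X and starts a fast looping timer calling UpdateParallax instead of using Tick.
; Each update shifts the far, mid and near components along X by the player's travel times a per-layer factor, keeping fixed Y and Z offsets for layering.
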(event EventBeginPlay
  (Variables|Default|SetPlayerStartX (.X (Math|Vector|BreakVector (Transformation|GetActorLocation (Game|GetPlayerCharacter 0)))))
  (Utilities|Time|SetTimerbyFunctionName 0 "UpdateParallax" 0.01 true))

(event Collision|EventActorBeginOverlap
  (params (OtherActor :type Actor%20Object%20Reference)))

(event EventTick
  (params (DeltaSeconds :type Float%20%28single-precision%29)))

(fn ConstructionScript)

(fn UpdateParallax
  (Variables|Default|SetDeltaX (- (.X (Math|Vector|BreakVector (Transformation|GetActorLocation (Game|GetPlayerCharacter 0)))) (Variables|Default|GetPlayerStartX)))
  (Utilities|FlowControl|Sequence
    (:then_0
      (Transformation|SetRelativeLocation (Variables|Default|GetScene) (Math|Vector|MakeVector (+ (Variables|Default|GetXStart) (* (Variables|Default|GetDeltaX) (Variables|Default|GetFarBG))) (+ (Variables|Default|GetYStart) -2e+02) (Variables|Default|GetZStart)) false true))
    (:then_1
      (Transformation|SetRelativeLocation (Variables|Default|GetSP_Mid) (Math|Vector|MakeVector (+ (Variables|Default|GetXStart) (* (Variables|Default|GetDeltaX) (Variables|Default|GetMidBG))) (+ (Variables|Default|GetYStart) -1e+02) (- (Variables|Default|GetZStart) 1e+02)) false true))
    (:then_2
      (Transformation|SetRelativeLocation (Variables|Default|GetSP_Near) (Math|Vector|MakeVector (+ (Variables|Default|GetXStart) (* (Variables|Default|GetDeltaX) (Variables|Default|GetNearBG))) (Variables|Default|GetYStart) (Variables|Default|GetZStart)) false true))))